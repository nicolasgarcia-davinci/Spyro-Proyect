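; BP_HUDUpdater tracks the player's money and relays money and life changes through event dispatchers, apparently for the HUD.
; MoneyBag resets to zero on BeginPlay, then Get Money adds to it and Pay The Toll subtracts with a clamp against going negative, each broadcasting the new total.
; Live Display Update stores nothing and simply rebroadcasts the lives value it receives.
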(event `self.ReceiveBeginPlay`
  (set `self.Money Bag` 0.0))

(fn `Get Money`
  (params (`Add Money` :type "Float (double-precision)"))
  (bind _output_get (set `self.Money Bag` (+ (`self.Money Bag`) `Add Money`)))
  (`self.ADD MONEY` _output_get))

(fn `Live Display Update`
  (params (Lives :type "Float (double-precision)"))
  (`self.UPDATE LIFE DISPLAY` Lives))

(fn `Pay The Toll`
  (params (Bill :type "Float (double-precision)"))
  (bind _output_get (set `self.Money Bag` (`KismetMathLibrary.FClamp` (- (`self.Money Bag`) Bill) 0.0 999999999999.0)))
  (`self.PAY` _output_get))