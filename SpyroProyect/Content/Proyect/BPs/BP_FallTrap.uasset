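; BP_FallTrap is a trap that drops away when a BP_Ninja overlaps its Box, then returns to its start position.
; BeginPlay stores the start position and an end position 1000 units below it.
; The AntesDeCaer timeline nudges the actor down by its Anticipation value each update with sweep, then snaps it to the end position.
; The DespuesDeCaer timeline serves as a delay before snapping it back.
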(event `self.ReceiveBeginPlay`
  ;[1 1 1] Sep Positions
  (bind _output_get (set `self.SPos` (`self.K2_GetActorLocation` self)))
  (set `self.EPos` (+ _output_get (0.0 0.0 -1000.0))))

(event `self.Box.OnComponentBeginOverlap`
  (params (OverlappedComponent :type "PrimitiveComponent Object Reference") (OtherActor :type "Actor Object Reference") (OtherComp :type "PrimitiveComponent Object Reference") (OtherBodyIndex :type Integer) (bFromSweep :type Boolean) (SweepResult :type "HitResult Structure (by ref)"))
  (bind (_returnvalue_x _returnvalue_y _returnvalue_z) (`KismetMathLibrary.BreakVector` (`self.K2_GetActorLocation` self)))
  ;[1 1 1] Fall And Return
  (cast `/Game/ThirdPerson/Blueprints/BP_Ninja` OtherActor)
  (bind (_direction _anticipation) (`Timeline|Antes de Caer` :!via `PlayFromStart`)
    (:`Update`
      (`self.K2_SetActorLocation` self (`KismetMathLibrary.MakeVector` _returnvalue_x _returnvalue_y (- _returnvalue_z _anticipation)) true false))
    (:`Finished`
      (`self.K2_SetActorLocation` self (`self.EPos`) false false)
      (`Timeline|Despues de Caer` :!via `PlayFromStart`
        (:`Finished`
          (`self.K2_SetActorLocation` self (`self.SPos`) false false))))))

(fn `UserConstructionScript`)