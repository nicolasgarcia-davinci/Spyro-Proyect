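; BP_Ork is an enemy that damages BP_Ninja on contact, or gets knocked away if the ninja is charging.
; A charged hit applies a one-time force to its Cone, then destroys the Ork when the DIETIME timeline ends.
; While the ninja stays in PlayerINRange, the TrapPrep timeline runs, spawning a BP_StikyTrap at the Cone's relative location on completion; leaving range stops it.
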(event `self.Cone.OnComponentHit`
  (params (HitComponent :type "PrimitiveComponent Object Reference") (OtherActor :type "Actor Object Reference") (OtherComp :type "PrimitiveComponent Object Reference") (NormalImpulse :type "Vector Structure") (Hit :type "HitResult Structure (by ref)"))
  ;[1 1 1] Player Hit
  (bind _asbp_ninja (cast `/Game/ThirdPerson/Blueprints/BP_Ninja` OtherActor))
  (if (`/Game/ThirdPerson/Blueprints/BP_Ninja.Is Player Charging` _asbp_ninja)
    (`self.Fly Away`)
    (else
      (message `/Game/Proyect/InterFace/BPI_TakeDamga.Get Damage` _asbp_ninja -1.0))))

(event `/Game/Proyect/InterFace/BPI_Ork_Away.Fly Away`
  ;[1 1 1] Fly away
  (`/Engine/EditorBlueprintResources/StandardMacros.DoOnce` false
    (:`Completed`
      (`PrimitiveComponent.AddForce` (`self.Cone`) (`self.Push Force`) "None" false)
      (`Timeline|DIE TIME`
        (:`Finished`
          (`self.K2_DestroyActor`))))))

(event `self.PlayerINRange.OnComponentBeginOverlap`
  (params (OverlappedComponent :type "PrimitiveComponent Object Reference") (OtherActor :type "Actor Object Reference") (OtherComp :type "PrimitiveComponent Object Reference") (OtherBodyIndex :type Integer) (bFromSweep :type Boolean) (SweepResult :type "HitResult Structure (by ref)"))
  ;[1 1 1] Stiky Spawn
  (cast `/Game/ThirdPerson/Blueprints/BP_Ninja` OtherActor)
  (`Timeline|Trap Prep` :!via `PlayFromStart` :!label _label
    (:`Finished`
      (`|SpawnActorFromClass` "/Game/Proyect/BPs/BP_StikyTrap.BP_StikyTrap_C" (`KismetMathLibrary.Conv_VectorToTransform` (`SceneComponent.RelativeLocation` (`self.Cone`))) "Undefined" "MultiplyWithRoot" null null))))

(event `self.PlayerINRange.OnComponentEndOverlap`
  (params (OverlappedComponent :type "PrimitiveComponent Object Reference") (OtherActor :type "Actor Object Reference") (OtherComp :type "PrimitiveComponent Object Reference") (OtherBodyIndex :type Integer))
  ;[1 1 1] Stiky Spawn
  (cast `/Game/ThirdPerson/Blueprints/BP_Ninja` OtherActor)
  (goto _label :!via `Stop`))

(fn `UserConstructionScript`)