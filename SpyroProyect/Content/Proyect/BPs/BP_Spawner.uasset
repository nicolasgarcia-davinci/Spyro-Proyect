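; BP_Spawner is a one-shot trigger that spawns minions after a BP_Ninja has spent enough time inside its capsule.
; Capsule overlap plays a Timeline and leaving stops it, so progress resumes on re-entry rather than restarting.
; When the Timeline finishes, SpawnEnemy spawns the Minion class at every transform in the SpawnPos array, then the spawner destroys itself.
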(event `self.Capsule.OnComponentBeginOverlap`
  (params (OverlappedComponent :type "PrimitiveComponent Object Reference") (OtherActor :type "Actor Object Reference") (OtherComp :type "PrimitiveComponent Object Reference") (OtherBodyIndex :type Integer) (bFromSweep :type Boolean) (SweepResult :type "HitResult Structure (by ref)"))
  (cast `/Game/ThirdPerson/Blueprints/BP_Ninja` OtherActor)
  (`Timeline|Timeline` :!label _label
    (:`Finished`
      (`self.Spawn Enemy`)
      (`self.K2_DestroyActor`))))

(event `self.Capsule.OnComponentEndOverlap`
  (params (OverlappedComponent :type "PrimitiveComponent Object Reference") (OtherActor :type "Actor Object Reference") (OtherComp :type "PrimitiveComponent Object Reference") (OtherBodyIndex :type Integer))
  (cast `/Game/ThirdPerson/Blueprints/BP_Ninja` OtherActor)
  (goto _label :!via `Stop`))

(event `Spawn Enemy`
  (for _array_element (`self.Spawn Pos`)
    (`|SpawnActorFromClass` (`self.Minion`) _array_element "Undefined" "MultiplyWithRoot" null null)))

(fn `UserConstructionScript`)