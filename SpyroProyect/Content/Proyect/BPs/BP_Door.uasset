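; BP_Door is a gem-toll door that unlocks when BP_Ninja hits its Porton component with enough gems.
; It checks the ninja's BPGemUpdater MoneyBag against CostToOpenDor, then charges the toll, plays an unlock sound and destroys itself when the PreDie timeline finishes.
; Otherwise it prints a warning and plays a locked sound, using a DoOnce that a timeline resets to throttle repeated hits.
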(event `self.porton.OnComponentHit`
  (params (HitComponent :type "PrimitiveComponent Object Reference") (OtherActor :type "Actor Object Reference") (OtherComp :type "PrimitiveComponent Object Reference") (NormalImpulse :type "Vector Structure") (Hit :type "HitResult Structure (by ref)"))
  (bind _cost_to_open_dor (`self.Cost To Open Dor`))
  (bind _returnvalue (`SceneComponent.K2_GetComponentLocation` (`self.porton`)))
  (bind _asbp_ninja (cast `/Game/ThirdPerson/Blueprints/BP_Ninja` OtherActor))
  (bind _bp_gemupdater (`/Game/ThirdPerson/Blueprints/BP_Ninja.BP_GemUpdater` _asbp_ninja))
  (if (>= (`/Game/Proyect/InterFace/BP_HUDUpdater.Money Bag` _bp_gemupdater) _cost_to_open_dor)
    (`/Game/Proyect/InterFace/BP_HUDUpdater.Pay The Toll` _bp_gemupdater _cost_to_open_dor)
    (`GameplayStatics.PlaySoundAtLocation` "/Game/Proyect/Sounds/SFX/SW_Unlock.SW_Unlock" _returnvalue (struct) 1.0 1.0 0.0 null null null null)
    (`Timeline|Pre-Die`
      (:`Finished`
        (`self.K2_DestroyActor`)))
    (else
      (`/Engine/EditorBlueprintResources/StandardMacros.DoOnce` false :!label _label
        (:`Completed`
          (`KismetSystemLibrary.PrintString` "U Need More Gems To Open This Door")
          (`GameplayStatics.PlaySoundAtLocation` "/Game/Proyect/Sounds/SFX/SW_LockDoor.SW_LockDoor" _returnvalue (struct) 1.0 1.0 0.0 null null null null)
          (`Timeline|Timeline` :!via `PlayFromStart`
            (:`Finished`
              (goto _label :!via `Reset`))))))))

(fn `UserConstructionScript`)