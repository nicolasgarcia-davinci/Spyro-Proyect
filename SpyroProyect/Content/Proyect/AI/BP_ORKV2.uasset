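; BP_ORKV2 is an ork enemy that drops sticky traps while the ninja player is nearby and can be knocked away by a charge.
; AI perception writes the sensing result to the IsPlayerInRange blackboard key, while a separate overlap component runs the looping trap timer.
; A capsule hit from a charging ninja launches the ork, which later spawns a gem and destroys itself.
; Otherwise, contact marks it attacking and damages the ninja only once.
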(event `self.AIPerception.OnTargetPerceptionUpdated`
  (params (Actor :type "Actor Object Reference") (Stimulus :type "AIStimulus Structure"))
  ;[1 1 1] Perception
  (bind _asaicontroller (cast `AIController` (`self.GetController`)))
  (`BlackboardComponent.SetValueAsBool` (`AIController.Blackboard` _asaicontroller) "IsPlayerInRange" (`.bSuccessfullySensed` (break `AIStimulus` Stimulus))))

(event `self.CapsuleComponent.OnComponentHit`
  (params (HitComponent :type "PrimitiveComponent Object Reference") (OtherActor :type "Actor Object Reference") (OtherComp :type "PrimitiveComponent Object Reference") (NormalImpulse :type "Vector Structure") (Hit :type "HitResult Structure (by ref)"))
  ;[1 1 1] Charge Chaeck
  (bind _asbp_ninja (cast `/Game/ThirdPerson/Blueprints/BP_Ninja` OtherActor))
  (if (`/Game/ThirdPerson/Blueprints/BP_Ninja.Is Player Charging` _asbp_ninja)
    (set `self.isEnemyKnocked` true)
    (`GameplayStatics.PlaySoundAtLocation` "/Game/Proyect/Sounds/SFX/SW_EnemyDamage.SW_EnemyDamage" (`SceneComponent.K2_GetComponentLocation` (`self.Mesh`)) (struct) 1.0 1.0 0.0 null null null null)
    (`self.Fly Away`)
    (else
      (set `self.isEnemyAttacking` true)
      (`/Engine/EditorBlueprintResources/StandardMacros.DoOnce` false
        (:`Completed`
          (message `/Game/Proyect/InterFace/BPI_TakeDamga.Get Damage` _asbp_ninja -1.0))))))

(event `/Game/Proyect/InterFace/BPI_Ork_Away.Fly Away`
  ;[1 1 1] Fly
  (`/Engine/EditorBlueprintResources/StandardMacros.DoOnce` false
    (:`Completed`
      (`PrimitiveComponent.AddForce` (`self.CapsuleComponent`) (`self.Launch Force`) "None" false)
      (`Timeline|TimeTo Die`
        (:`Finished`
          (`|SpawnActorFromClass` (`self.Gem`) (`KismetMathLibrary.Conv_VectorToTransform` (`SceneComponent.K2_GetComponentLocation` (`self.CapsuleComponent`))) "Undefined" "MultiplyWithRoot" null null)
          (`self.K2_DestroyActor`))))))

(event `self.Player In Range.OnComponentBeginOverlap`
  (params (OverlappedComponent :type "PrimitiveComponent Object Reference") (OtherActor :type "Actor Object Reference") (OtherComp :type "PrimitiveComponent Object Reference") (OtherBodyIndex :type Integer) (bFromSweep :type Boolean) (SweepResult :type "HitResult Structure (by ref)"))
  ;[1 1 1] Trap Spawner
  (cast `/Game/ThirdPerson/Blueprints/BP_Ninja` OtherActor)
  (`Timeline|Trap Time` :!via `PlayFromStart` :!label _label
    (:`Finished`
      (`GameplayStatics.PlaySoundAtLocation` "/Game/Proyect/Sounds/SFX/SW_Trap.SW_Trap" (`SceneComponent.K2_GetComponentLocation` (`self.CapsuleComponent`)) (struct) 1.0 1.0 0.0 null null null null)
      (`|SpawnActorFromClass` "/Game/Proyect/BPs/BP_StikyTrap.BP_StikyTrap_C" (`KismetMathLibrary.Conv_VectorToTransform` (`SceneComponent.RelativeLocation` (`self.CapsuleComponent`))) "Undefined" "MultiplyWithRoot" null null)
      (goto _label :!via `PlayFromStart`))))

(event `self.Player In Range.OnComponentEndOverlap`
  (params (OverlappedComponent :type "PrimitiveComponent Object Reference") (OtherActor :type "Actor Object Reference") (OtherComp :type "PrimitiveComponent Object Reference") (OtherBodyIndex :type Integer))
  ;[1 1 1] Trap Spawner
  (cast `/Game/ThirdPerson/Blueprints/BP_Ninja` OtherActor)
  (goto _label :!via `Stop`))

(fn `UserConstructionScript`)